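; Pickup skill actor for a dance gun, which a third-person character collects by walking into its box trigger.
; If the character holds no skill, it registers itself as the current skill, snaps to the left-hand socket, plays a sound and destroys its pickup cube and trigger.
; Otherwise it only prints a warning.
; BeginSkill is a placeholder that prints a shooting message without firing anything.
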(event OnComponentBeginOverlap(Box)
  (params (OverlappedComponent :type Primitive%20Component%20Object%20Reference) (OtherActor :type Actor%20Object%20Reference) (OtherComp :type Primitive%20Component%20Object%20Reference) (OtherBodyIndex :type Integer) (bFromSweep :type Boolean) (SweepResult :type Hit%20Result%20Structure%20%28by%20ref%29))
  ;[1 1 1] grab the skill, unless we already have a skill
  (bind _asbp_third_person_character (Utilities|Casting|CastToBP_ThirdPersonCharacter OtherActor))
  (bind _output_get (Variables|Default|SetAs%20BP%20Third%20Person%20Character _asbp_third_person_character))
  (Variables|/Game/ThirdPerson/Blueprints/BP_ThirdPersonCharacter.BP_ThirdPersonCharacter_C|GetCurrentSKill _output_get
    (:then
      (Development|PrintString "You're already holding a skill!"))
    (:else
      (Variables|/Game/ThirdPerson/Blueprints/BP_ThirdPersonCharacter.BP_ThirdPersonCharacter_C|SetCurrentSKill _output_get self)
      (Transformation|AttachComponentToComponent (Variables|/Script/Engine.Character|GetMesh _output_get) "lhand" "SnapToTarget" "SnapToTarget" "SnapToTarget" true) ; attach this skill to the player's left hand
      (Development|PrintString "holding DANCE GUN")
      (Audio|PlaySoundatLocation "/Game/Audio/bleepbloops1.bleepbloops1" (Transformation|GetWorldLocation (Variables|Default|GetDefaultSceneRoot)) "0, 0, 0" 1.0 1.0 0.0 0 0 0 0)
      (Components|DestroyComponent (Variables|Default|GetCube)))))

(event EventBeginSkill
  (Development|PrintString "SHOOTING BULLET"))

(fn ConstructionScript)